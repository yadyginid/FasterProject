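; Goblin AI Blueprint that plays a brief gold effect when its OnTakenItem event fires.
; One second after BeginPlay, only instances without authority bind to OnTakenItem, so the effect is cosmetic and never plays on the server.
; The handler shows and activates the NEGold3 effect component, then hides and deactivates it after a short delay.
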(event Custom|OnTakenItem_Event
  (bind _ne_gold3 (Variables|Default|GetNE_gold3))
  (Rendering|SetVisibility (Variables|Default|GetNE_gold3) true false)
  (Components|Activation|Activate (Variables|Default|GetNE_gold3) false)
  (Utilities|FlowControl|Delay 1.0)
  (Rendering|SetVisibility _ne_gold3 false false)
  (Components|Activation|Deactivate _ne_gold3))

(event EventBeginPlay
  (Utilities|FlowControl|Delay 1.0)
  (if (not (Ability|HasAuthority))
    (EventDispatchers|AssignOnTakenItem self (delegate Custom|OnTakenItem_Event))))

(fn ConstructionScript)